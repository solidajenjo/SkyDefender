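; Flying invader ship that destroys building walls, switching to attack the player or other ships when the Level flags KillPlayer or CivilWar.
; After a random falling delay, it picks a random wall from Level, flies to its fire position, turns and spawns a projectile.
; Tick drives physics-velocity movement, sweeping yaw line traces for a clear heading when the target is blocked.
; HasTarget also switches body and particle materials between red and default.
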(event `self.ReceiveTick`
  (params (DeltaSeconds :type "Float (single-precision)"))
  (bind _alpharot (`self.alphaRot`))
  (bind _scene (`self.Scene`))
  (bind _cube (`self.Cube`))
  (bind _scene_2 (`self.Scene`))
  (bind _level (`self.Level`))
  (bind _targetship (`self.targetShip`))
  (bind _target (`self.target`))
  (bind _scene_3 (`self.Scene`))
  (bind _targetfireposition (`self.targetFirePosition`))
  (bind _returnvalue (`SceneComponent.K2_GetComponentLocation` (`self.Cube`)))
  (bind _returnvalue_2 (`SceneComponent.K2_GetComponentLocation` _cube))
  (bind (_relativerotation_roll _relativerotation_pitch _relativerotation_yaw) (`KismetMathLibrary.BreakRotator` (`SceneComponent.RelativeRotation` _scene_2)))
  (bind _returnvalue_3 (`SceneComponent.K2_GetComponentLocation` (`/Game/Blueprints/BP_BuildingDestroyer.Cube` _targetship)))
  (bind (_returnvalue_roll _returnvalue_pitch _returnvalue_yaw) (`KismetMathLibrary.BreakRotator` (`KismetMathLibrary.FindLookAtRotation` (`SceneComponent.K2_GetComponentLocation` _scene_2) _targetfireposition)))
  ;[1 1 1] Init - State Logic
  ;[1 1 1] Debug
  (if (`self.debug`)
    (`self.DebugLines` _returnvalue _target _target _returnvalue (`self.newDestination`) (`self.targetFirePosition`)))
  (`self.MaterialsHandler`
    (:`then`
      _)
    (:`then2`
      _))
  (if (`/Game/Blueprints/BP_Level.civilWar` _level)
    ;[1 1 1] Civil War - Kill player Management
    (`PrimitiveComponent.SetCollisionResponseToChannel` (`self.Cube`) "ECC_Visibility" "ECR_Block")
    (if (`KismetSystemLibrary.IsValid` _targetship)
      (set `self.target` _returnvalue_3)
      (set `self.targetFirePosition` _returnvalue_3)
      (if (`self.hasTarget`) :!label _label
        (`SceneComponent.K2_SetWorldRotation` _scene (`KismetMathLibrary.FindLookAtRotation` (`SceneComponent.K2_GetComponentLocation` _scene) (`self.target`)) false false)
        (`|ExecutionSequence`
          (:`then_0`
            (`KismetSystemLibrary.Delay` 2.0)
            (`|SpawnActorFromClass` "/Game/Blueprints/BP_Projectile.BP_Projectile_C" (`SceneComponent.K2_GetComponentToWorld` _scene) "Undefined" "OverrideRootScale" null (`self.Level`) self "/Game/Particles/MT_Projectile_Inst.MT_Projectile_Inst" null))
          (:`then_1`
            _)))
      ;[1 1 1] Movement Management
      (if (`self.hasTarget`) :!label _label_2
        (`self.movement`)
        (else
          (`self.movement`)
          (`KismetSystemLibrary.Delay` (`KismetMathLibrary.RandomFloatInRange` 0.5 1.0))))
      (set `self.hasTarget` false)
      (bind _outhits (`KismetSystemLibrary.LineTraceMulti` (`SceneComponent.K2_GetComponentLocation` (`self.Cube`)) (`self.targetFirePosition`) "TraceTypeQuery1"))
      (for _array_element _outhits
        (if (< (`KismetMathLibrary.VSize` (- (`.ImpactPoint` (`GameplayStatics.BreakHitResult` _array_element)) (`self.targetFirePosition`))) 40.0)
          (set `self.hasTarget` true)
          (set `self.newDestination` (`self.targetFirePosition`))))
      (if (not (`self.hasTarget`))
        (set `self.newDestination` _targetfireposition)
        (`SceneComponent.K2_SetWorldRotation` _scene_2 (`KismetMathLibrary.MakeRotator` _returnvalue_roll _returnvalue_pitch _returnvalue_yaw) false false)
        (set `self.rotZ` _relativerotation_yaw)
        (for _index (range 361)
          (bind _returnvalue_4 (`self.rotateRau` (`KismetMathLibrary.Conv_IntToDouble` _index)))
          (bind _output_get (set `self.newDestination` _returnvalue_4))
          (bind _outhit (`KismetSystemLibrary.LineTraceSingle` :`Start` (`SceneComponent.K2_GetComponentLocation` (`self.Cube`)) :`End` _output_get :`TraceChannel` "TraceTypeQuery1" :`bTraceComplex` true :`DrawTime` 1.0))
          (if (`GameplayStatics.BreakHitResult` _outhit)
            (bind _returnvalue_5 (`self.rotateRau` (`KismetMathLibrary.Conv_IntToDouble` (* _index -1))))
            (bind _output_get_2 (set `self.newDestination` _returnvalue_5))
            (bind _outhit_2 (`KismetSystemLibrary.LineTraceSingle` :`Start` (`SceneComponent.K2_GetComponentLocation` (`self.Cube`)) :`End` _output_get_2 :`TraceChannel` "TraceTypeQuery1" :`bTraceComplex` true :`DrawTime` 1.0))
            (if (not (`GameplayStatics.BreakHitResult` _outhit_2))
              (break))
            (else
              (break)))))
      (else
        (`/Game/Blueprints/BP_Level.pickRandomShip` (`self.Level`) self)))
    (else
      (`PrimitiveComponent.SetCollisionResponseToChannel` (`self.Cube`) "ECC_Visibility" "ECR_Ignore")
      (if (`/Game/Blueprints/BP_Level.killPlayer` _level)
        (`PrimitiveComponent.SetCollisionResponseToChannel` (`self.Cube`) "ECC_Visibility" "ECR_Block")
        (bind _output_get_3 (set `self.target` (`self.K2_GetActorLocation` (`/Game/Blueprints/BP_Level.Player` (`self.Level`)))))
        (set `self.targetFirePosition` _output_get_3)
        (goto _label)
        (else
          (`PrimitiveComponent.SetCollisionResponseToChannel` (`self.Cube`) "ECC_Visibility" "ECR_Ignore")
          (if (`self.firing`)
            ;[1 1 1] Destroy Wall
            (`KismetSystemLibrary.LineTraceSingle` :`Start` _returnvalue_2 :`End` (+ (* (`SceneComponent.GetForwardVector` _cube) 1000.0) _returnvalue_2) :`TraceChannel` "TraceTypeQuery1" :`DrawTime` 1.0)
            (if (>= _alpharot 0.9)
              (`SceneComponent.K2_SetWorldRotation` _scene_3 (`KismetMathLibrary.FindLookAtRotation` (`SceneComponent.K2_GetComponentLocation` _scene_3) (`self.target`)) false false)
              (`|SpawnActorFromClass` "/Game/Blueprints/BP_Projectile.BP_Projectile_C" (`SceneComponent.K2_GetComponentToWorld` _scene_3) "Undefined" "OverrideRootScale" null (`self.Level`) self "/Game/Particles/MT_Projectile_Inst.MT_Projectile_Inst" null)
              (set `self.firing` false)
              (`self.pickRandomWall`)
              (else
                (set `self.alphaRot` (`KismetMathLibrary.FClamp` (+ _alpharot (`GameplayStatics.GetWorldDeltaSeconds`))))
                (`SceneComponent.K2_SetWorldRotation` _cube (`KismetMathLibrary.RLerp` (`SceneComponent.K2_GetComponentRotation` _cube) (`KismetMathLibrary.FindLookAtRotation` _returnvalue_2 (`self.target`)) _alpharot true) false false)))
            (elif (and (< (`KismetMathLibrary.VSize` (- (`SceneComponent.K2_GetComponentLocation` (`self.Cube`)) (`self.targetFirePosition`))) 20.0) (`self.hasTarget`))
              (set `self.firing` true)
              (`PrimitiveComponent.SetPhysicsLinearVelocity` (`self.Cube`) (0.0 0.0 0.0) false "None")
              (set `self.alphaRot` 0.0)
              (elif (<= (`self.fallingTimer`) 0.0)
                (if (`self.initialized`)
                  (goto _label_2)
                  (else
                    (`PrimitiveComponent.SetEnableGravity` (`self.Cube`) false)
                    (`PrimitiveComponent.SetPhysicsLinearVelocity` (`self.Cube`) (0.0 0.0 0.0) false "None")
                    (set `self.initialized` true)
                    (`self.pickRandomWall`)))
                (else
                  (`self.decTimer`))))))))))

(event `self.ReceiveBeginPlay`
  (set `self.fallingTimer` (`KismetMathLibrary.RandomFloatInRange` 2.0 4.0)))

(event `ShipDestroyed`
  ;[1 1 1] Debug
  (`KismetSystemLibrary.PrintString` "Ship Destroyed"))

(fn `angleBetween`
  (params (A :type "Vector Structure") (A2 :type "Vector Structure"))
  (returns (ReturnValue :type "Float (double-precision)"))
  (return (`KismetMathLibrary.DegAcos` (`KismetMathLibrary.Dot_VectorVector` (`KismetMathLibrary.Normal` A) (`KismetMathLibrary.Normal` A2)))))

(fn `calculateNewPath`
  (params (self2 :type "GridNav3D Object Reference") (originWorld :type "Vector Structure"))
  (`self.pickRandomWall`))

(fn `decTimer`
  (set `self.fallingTimer` (- (`self.fallingTimer`) (`GameplayStatics.GetWorldDeltaSeconds`))))

(fn `movement`
  (locals (speed :type "Float (double-precision)" :default 200.0))
  (bind _cube (`self.Cube`))
  (bind (_target_x _target_y _target_z) (`KismetMathLibrary.BreakVector` (`self.target`)))
  (bind _cube_2 (`self.Cube`))
  (bind _returnvalue (`SceneComponent.K2_GetComponentLocation` _cube_2))
  (bind (_returnvalue_x _returnvalue_y _returnvalue_z) (`KismetMathLibrary.BreakVector` (`SceneComponent.K2_GetComponentLocation` _cube)))
  (`PrimitiveComponent.SetPhysicsLinearVelocity` _cube_2 (* (`KismetMathLibrary.Normal` (- (`self.newDestination`) _returnvalue)) (`local.speed`)) false "None")
  (if (> _target_z _returnvalue_z)
    (`PrimitiveComponent.AddImpulse` _cube (0.0 0.0 1000.0) "None" false)
    (else
      (`PrimitiveComponent.AddImpulse` _cube (0.0 0.0 -1000.0) "None" false)))
  (`SceneComponent.K2_SetWorldRotation` _cube_2 (`KismetMathLibrary.RLerp` (`SceneComponent.K2_GetComponentRotation` _cube_2) (`KismetMathLibrary.FindLookAtRotation` _returnvalue (`self.newDestination`)) 0.1 true) false false))

(fn `pickRandomWall`
  (bind _walls (`/Game/Blueprints/BP_Level.Walls` (`self.Level`)))
  (bind _returnvalue (`KismetArrayLibrary.Array_Length` _walls))
  (if (== _returnvalue 0)
    (`self.K2_DestroyActor`)
    (else
      (bind _result (`/Engine/EditorBlueprintResources/StandardMacros.DecrementInt` _returnvalue)
        (:`  `
          (bind _output_get (set `self.targetST` (`|GetArrayItem` _walls (`KismetMathLibrary.RandomIntegerInRange` 0 _result))))
          (bind _output_get_2 (set `self.target` (break `/Game/Blueprints/ST_Wall` _output_get)))
          (set `self.newDestination` _output_get_2)
          (set `self.targetFirePosition` (`.firePosition_4_E1770D8C46E40D0EC0EBA38CCC10C2C8` (break `/Game/Blueprints/ST_Wall` _output_get)))
          (set `self.hasTarget` true)
          (return))))))

(fn `rotateRau`
  (params (AngleDeg :type "Float (double-precision)"))
  (returns (ReturnValue :type "Vector Structure"))
  (bind _scene (`self.Scene`))
  (`SceneComponent.K2_SetRelativeRotation` _scene (`KismetMathLibrary.MakeRotator` 0.0 0.0 (+ AngleDeg (`self.rotZ`))) false false)
  (return (* (`SceneComponent.GetForwardVector` _scene) 10000.0)))

(fn `UserConstructionScript`)