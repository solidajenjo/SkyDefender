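; BP_Player is a player-controlled flying actor that rolls, pitches, accelerates and fires projectiles.
; Axis inputs rotate it locally and adjust Speed using delta time, while Tick sweeps it along its forward vector by the raw Speed per frame, then clamps Speed.
; Fire spawns BP_Projectile at the ProjectileSpawner transform.
; Sphere hits nudge the actor along the hit normal and subtract CollisionFriction from Speed.
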(event `InputAxis|LEFT_Axis`
  (params (AxisValue :type "Float (single-precision)"))
  (`self.K2_AddActorLocalRotation` (`KismetMathLibrary.MakeRotator` (* AxisValue (`self.rotSpeed`) (`GameplayStatics.GetWorldDeltaSeconds`)))))

(event `InputAxis|UP_Axis`
  (params (AxisValue :type "Float (single-precision)"))
  (`self.K2_AddActorLocalRotation` (`KismetMathLibrary.MakeRotator` 0.0 (* AxisValue (`self.rotSpeed`) (`GameplayStatics.GetWorldDeltaSeconds`)))))

(event `self.ReceiveTick`
  (params (DeltaSeconds :type "Float (single-precision)"))
  (`self.K2_AddActorWorldOffset` (* (`self.GetActorForwardVector`) (`self.speed`)) true true)
  (set `self.speed` (`KismetMathLibrary.FClamp` (`self.speed`) 0.0 (`self.maxSpeed`))))

(event `InputAction|Fire`
  (params (Key :type "Key Structure"))
  (:`Pressed`
    (`|SpawnActorFromClass` "/Game/Blueprints/BP_Projectile.BP_Projectile_C" (`SceneComponent.K2_GetComponentToWorld` (`self.ProjectileSpawner`)) "Undefined" "OverrideRootScale" null null)))

(event `self.Sphere.OnComponentHit`
  (params (HitComponent :type "PrimitiveComponent Object Reference") (OtherActor :type "Actor Object Reference") (OtherComp :type "PrimitiveComponent Object Reference") (NormalImpulse :type "Vector Structure") (Hit :type "HitResult Structure (by ref)"))
  (`self.K2_AddActorWorldOffset` Hit_Normal true true)
  (set `self.speed` (- (`self.speed`) (`self.collisionFriction`))))

(event `InputAxis|Acceleration_Axis`
  (params (AxisValue :type "Float (single-precision)"))
  (if (!= AxisValue 0.0)
    (set `self.speed` (+ (* AxisValue (`self.acceleration`) (`GameplayStatics.GetWorldDeltaSeconds`)) (`self.speed`)))))

(fn `UserConstructionScript`)