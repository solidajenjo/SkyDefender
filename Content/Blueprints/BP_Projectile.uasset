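; Physics-driven projectile that destroys BP_BuildingDestroyer ships on hit and reports the kill to its Parent.
; BeginPlay launches the sphere with a forward impulse and applies its material; Tick counts down LifeTimer to destroy it.
; Other hits, any overlap, or a kill with a valid Parent trigger a burst, radial impulse and self-destruction.
; A swept manual-movement node remains but never runs.
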(event `self.ReceiveBeginPlay`
  (bind _material (`self.material`))
  (`PrimitiveComponent.AddImpulse` (`self.Sphere`) (* (`self.GetActorForwardVector`) (`self.speed`)) "None" false)
  (`PrimitiveComponent.SetMaterial` (`self.ParticleSystem`) 0 _material)
  (`PrimitiveComponent.SetMaterial` (`self.Sphere`) 0 _material))

(event `self.ReceiveTick`
  (params (DeltaSeconds :type "Float (single-precision)"))
  (bind _output_get (set `self.lifeTimer` (- (`self.lifeTimer`) (`GameplayStatics.GetWorldDeltaSeconds`))))
  (if (<= _output_get 0.0)
    (`self.K2_DestroyActor`)))

(event `self.Sphere.OnComponentHit`
  (params (HitComponent :type "PrimitiveComponent Object Reference") (OtherActor :type "Actor Object Reference") (OtherComp :type "PrimitiveComponent Object Reference") (NormalImpulse :type "Vector Structure") (Hit :type "HitResult Structure (by ref)"))
  (bind _parent (`self.parent`))
  (bind _asbp_building_destroyer (cast `/Game/Blueprints/BP_BuildingDestroyer` Hit_HitActor)
    (:`then`
      (bind _returnvalue (`SceneComponent.K2_GetComponentLocation` (`/Game/Blueprints/BP_BuildingDestroyer.Cube` _asbp_building_destroyer)))
      (`GameplayStatics.SpawnEmitterAtLocation` "/Game/Particles/PT_Invader_Burst_Blue.PT_Invader_Burst_Blue" _returnvalue (struct) (2.0 2.0 2.0))
      (`GameplayStatics.SpawnEmitterAtLocation` "/Game/Particles/PT_Invader_Burst_Red.PT_Invader_Burst_Red" _returnvalue (struct) (2.0 2.0 2.0))
      (`self.K2_DestroyActor` _asbp_building_destroyer)
      (if (`KismetSystemLibrary.IsValid` _parent)
        (`/Game/Blueprints/BP_BuildingDestroyer.ShipDestroyed` _parent)
        (`GameplayStatics.SpawnEmitterAtLocation` "/Game/Particles/PT_projectileBurst.PT_projectileBurst" (`SceneComponent.K2_GetComponentLocation` (`self.Scene`)) :!label _label)
        (`RadialForceComponent.FireImpulse` (`self.RadialForce`))
        (`self.K2_DestroyActor`)))
    (:`CastFailed`
      (goto _label))))

(event `self.Sphere.OnComponentBeginOverlap`
  (params (OverlappedComponent :type "PrimitiveComponent Object Reference") (OtherActor :type "Actor Object Reference") (OtherComp :type "PrimitiveComponent Object Reference") (OtherBodyIndex :type Integer) (bFromSweep :type Boolean) (SweepResult :type "HitResult Structure (by ref)"))
  (goto _label))

(fn `UserConstructionScript`)