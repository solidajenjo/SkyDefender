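; BP_Wall is a wall actor with four destructible sections, each paired with a scene point stored as its fire position.
; On BeginPlay it records each section's positions, broken flag and component in a struct and adds it to WallsPositions.
; Fracturing a section turns it gray and flags its individual struct variable as broken, without writing back to the array.
; The SetWall helper is an unwired stub.
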(event `self.ReceiveBeginPlay`
  (bind _destructible (`self.Destructible`))
  (bind _destructible3 (`self.Destructible3`))
  (bind _destructible1 (`self.Destructible1`))
  (bind _destructible2 (`self.Destructible2`))
  (bind _output_get (set `self.Wall_0` (make `/Game/Blueprints/ST_Wall` (`SceneComponent.K2_GetComponentLocation` _destructible) (`SceneComponent.K2_GetComponentLocation` (`self.Scene`)) false _destructible)))
  (`KismetArrayLibrary.Array_Add` (`self.wallsPositions`) _output_get)
  (bind _output_get_2 (set `self.Wall_1` (make `/Game/Blueprints/ST_Wall` (`SceneComponent.K2_GetComponentLocation` _destructible1) (`SceneComponent.K2_GetComponentLocation` (`self.Scene1`)) false _destructible1)))
  (`KismetArrayLibrary.Array_Add` (`self.wallsPositions`) _output_get_2)
  (bind _output_get_3 (set `self.Wall_2` (make `/Game/Blueprints/ST_Wall` (`SceneComponent.K2_GetComponentLocation` _destructible2) (`SceneComponent.K2_GetComponentLocation` (`self.Scene2`)) false _destructible2)))
  (`KismetArrayLibrary.Array_Add` (`self.wallsPositions`) _output_get_3)
  (bind _output_get_4 (set `self.Wall_3` (make `/Game/Blueprints/ST_Wall` (`SceneComponent.K2_GetComponentLocation` _destructible3) (`SceneComponent.K2_GetComponentLocation` (`self.Scene3`)) false _destructible3)))
  (`KismetArrayLibrary.Array_Add` (`self.wallsPositions`) _output_get_4))

(event `self.Destructible.OnComponentFracture`
  (params (HitPoint :type "Vector Structure (by ref)") (HitDirection :type "Vector Structure (by ref)"))
  (bind (_wall_0_wallposition _wall_0_fireposition) (break `/Game/Blueprints/ST_Wall` (`self.Wall_0`)))
  (`PrimitiveComponent.SetMaterial` (`self.Destructible`) 0 "/Game/Flying/Meshes/GrayMaterial.GrayMaterial")
  (set `self.Wall_0` (make `/Game/Blueprints/ST_Wall` _wall_0_wallposition _wall_0_fireposition true)))

(event `self.Destructible1.OnComponentFracture`
  (params (HitPoint :type "Vector Structure (by ref)") (HitDirection :type "Vector Structure (by ref)"))
  (bind (_wall_1_wallposition _wall_1_fireposition) (break `/Game/Blueprints/ST_Wall` (`self.Wall_1`)))
  (`PrimitiveComponent.SetMaterial` (`self.Destructible1`) 0 "/Game/Flying/Meshes/GrayMaterial.GrayMaterial")
  (set `self.Wall_1` (make `/Game/Blueprints/ST_Wall` _wall_1_wallposition _wall_1_fireposition true)))

(event `self.Destructible2.OnComponentFracture`
  (params (HitPoint :type "Vector Structure (by ref)") (HitDirection :type "Vector Structure (by ref)"))
  (bind (_wall_2_wallposition _wall_2_fireposition) (break `/Game/Blueprints/ST_Wall` (`self.Wall_2`)))
  (`PrimitiveComponent.SetMaterial` (`self.Destructible2`) 0 "/Game/Flying/Meshes/GrayMaterial.GrayMaterial")
  (set `self.Wall_2` (make `/Game/Blueprints/ST_Wall` _wall_2_wallposition _wall_2_fireposition true)))

(event `self.Destructible3.OnComponentFracture`
  (params (HitPoint :type "Vector Structure (by ref)") (HitDirection :type "Vector Structure (by ref)"))
  (bind (_wall_3_wallposition _wall_3_fireposition) (break `/Game/Blueprints/ST_Wall` (`self.Wall_3`)))
  (`PrimitiveComponent.SetMaterial` (`self.Destructible3`) 0 "/Game/Flying/Meshes/GrayMaterial.GrayMaterial")
  (set `self.Wall_3` (make `/Game/Blueprints/ST_Wall` _wall_3_wallposition _wall_3_fireposition true)))

(fn `setWall`
  (params (self2 :type "SceneComponent Object Reference") (self3 :type "SceneComponent Object Reference")))

(fn `UserConstructionScript`)