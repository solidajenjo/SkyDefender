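; BP_Building is an actor that procedurally assembles a building as a vertical stack of BP_Floor actors.
; On BeginPlay it spawns each floor at an even spacing along the root component's up vector, passing Level and Walls values into it.
; The floor count comes from a random range whose bounds are equal, so it is effectively fixed.
; The construction script is empty.
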(event `self.ReceiveBeginPlay`
  (bind _defaultsceneroot (`self.DefaultSceneRoot`))
  (bind _output_get (set `self.floorNum` (`KismetMathLibrary.RandomIntegerInRange` 20 20)))
  (for _index (range 1 (+ _output_get 1))
    (`|SpawnActorFromClass` "/Game/Blueprints/BP_Floor.BP_Floor_C" (`KismetMathLibrary.MakeTransform` (+ (`SceneComponent.K2_GetComponentLocation` _defaultsceneroot) (* (`SceneComponent.GetUpVector` _defaultsceneroot) (* _index 31.0)))) "Undefined" "OverrideRootScale" null (`self.Level`) (`self.Walls`) null)))

(fn `UserConstructionScript`)