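; BP_Level manages a battle level where building-destroyer bots attack buildings.
; BeginPlay spawns five buildings, pools their wall positions, creates a shared BP_AI and records four spawn points.
; Tick initializes the AI grid once, then spawns timed bots at random points until the count runs out.
; Destroyed walls reset bots targeting them, while Civil War and Kill Player inputs toggle modes, resetting all bots when switched off.
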(event `self.ReceiveBeginPlay`
  (bind (_returnvalue _returnvalue2) (`self.spawBuilding` (`self.Building`)))
  (set `self.BP_Building` _returnvalue)
  (bind _returnvalue_2 (`self.spawBuilding` (`self.Building2`)))
  (set `self.BP_Building_0` _returnvalue_2)
  (bind _returnvalue_3 (`self.spawBuilding` (`self.Building3`)))
  (set `self.BP_Building_1` _returnvalue_3)
  (bind _returnvalue_4 (`self.spawBuilding` (`self.Building4`)))
  (set `self.BP_Building_2` _returnvalue_4)
  (bind _returnvalue_5 (`self.spawBuilding` (`self.Building5`)))
  (set `self.BP_Building_3` _returnvalue_5)
  (bind _returnvalue_6 (`|SpawnActorFromClass` "/Game/Blueprints/BP_AI.BP_AI_C" _returnvalue2 "Undefined" "OverrideRootScale" null null))
  (set `self.AI_BP_Var` _returnvalue_6)
  (`self.initSpawns` (`self.Spawn3`))
  (`self.initSpawns` (`self.Spawn2`))
  (`self.initSpawns` (`self.Spawn4`))
  (`self.initSpawns` (`self.Spawn`))
  (bind _asflying_pawn (cast `/Game/FlyingBP/Blueprints/FlyingPawn` (`GameplayStatics.GetPlayerPawn` 0)))
  (set `self.Player` _asflying_pawn))

(event `self.ReceiveTick`
  (params (DeltaSeconds :type "Float (single-precision)"))
  (bind _nbots (`self.nBots`))
  (bind _spawntimer (`self.spawnTimer`))
  (if (`self.scanComplete`)
    (if (>= _nbots 0)
      (if (<= _spawntimer 0.0) :!label _label
        (`self.buildingDestroyerSpawn`)
        (`/Engine/EditorBlueprintResources/StandardMacros.DecrementInt` _nbots)
        (else
          (`self.decTimer` _spawntimer))))
    (else
      (`GridNav3D.initGrid` (`self.AI_BP_Var`))
      (set `self.scanComplete` true)
      (goto _label))))

(event `WallDestroyed`
  (params (wall :type "/Game/Blueprints/ST_Wall Structure"))
  (for _array_element (`self.bots`)
    (if (`KismetSystemLibrary.IsValid` _array_element)
      (bind _targetst_wallposition (break `/Game/Blueprints/ST_Wall` (`/Game/Blueprints/BP_BuildingDestroyer.targetST` _array_element)))
      (if (== wall_wallPosition_2_0F5D242F4BA8B3EADAD2C3A96F107163 _targetst_wallposition :`ErrorTolerance` 1.0)
        (set `/Game/Blueprints/BP_BuildingDestroyer.initialized` false _array_element)))))

(event `InputAction|CivilWar`
  (params (Key :type "Key Structure"))
  (:`Pressed`
    (`KismetSystemLibrary.PrintString` "Civil Mode")
    (bind _output_get (set `self.civilWar` (not (`self.civilWar`))))
    (if (not _output_get)
      (for _array_element (`self.bots`) :!label _label_2
        (if (`KismetSystemLibrary.IsValid` _array_element)
          (set `/Game/Blueprints/BP_BuildingDestroyer.initialized` false _array_element))))))

(event `InputAction|KillPlayer`
  (params (Key :type "Key Structure"))
  (:`Pressed`
    (`KismetSystemLibrary.PrintString` "Kill Player")
    (bind _output_get (set `self.killPlayer` (not (`self.killPlayer`))))
    (if (not _output_get)
      (goto _label_2))))

(fn `buildingDestroyerSpawn`
  (bind _returnvalue (`|SpawnActorFromClass` "/Game/Blueprints/BP_BuildingDestroyer.BP_BuildingDestroyer_C" (`KismetMathLibrary.MakeTransform` (`|GetArrayItem` (`self.SpawnPositions`) (`KismetMathLibrary.RandomIntegerInRange` 0 3))) "Undefined" "OverrideRootScale" null null null null))
  (set `/Game/Blueprints/BP_BuildingDestroyer.AI` (`self.AI_BP_Var`) _returnvalue)
  (set `self.spawnTimer` (`self.spawnTime`))
  (set `/Game/Blueprints/BP_BuildingDestroyer.Level` self _returnvalue)
  (`KismetArrayLibrary.Array_Add` (`self.bots`) _returnvalue))

(fn `decTimer`
  (params (A :type "Float (double-precision)"))
  (set `self.spawnTimer` (- A (`GameplayStatics.GetWorldDeltaSeconds`))))

(fn `initSpawns`
  (params (self2 :type "SceneComponent Object Reference"))
  (`KismetArrayLibrary.Array_Add` (`self.SpawnPositions`) (`SceneComponent.K2_GetComponentLocation` self2)))

(fn `pickRandomShip`
  (params (caller :type "/Game/Blueprints/BP_BuildingDestroyer Object Reference"))
  (locals (done :type Boolean))
  (bind _bots (`self.bots`))
  (set `local.done` false)
  (while (not (`local.done`))
    (bind _result (`/Engine/EditorBlueprintResources/StandardMacros.DecrementInt` (`KismetArrayLibrary.Array_Length` _bots))
      (:`  `
        (bind _output (`|GetArrayItem` _bots (`KismetMathLibrary.RandomIntegerInRange` 0 _result)))
        (bind _output_get (set `local.done` (not (== caller _output))))
        (if _output_get
          (set `/Game/Blueprints/BP_BuildingDestroyer.targetShip` _output caller))))))

(fn `spawBuilding`
  (params (self2 :type "SceneComponent Object Reference"))
  (returns (ReturnValue :type "/Game/Blueprints/BP_Building Object Reference") (ReturnValue2 :type "Transform Structure"))
  (bind _returnvalue (`SceneComponent.K2_GetComponentToWorld` self2))
  (bind _returnvalue_2 (`|SpawnActorFromClass` "/Game/Blueprints/BP_Building.BP_Building_C" _returnvalue "Undefined" "OverrideRootScale" null self null))
  (`KismetArrayLibrary.Array_Append` (`self.Walls`) (`/Game/Blueprints/BP_Building.wallPositions` _returnvalue_2))
  (return _returnvalue_2 _returnvalue))

(fn `UserConstructionScript`)